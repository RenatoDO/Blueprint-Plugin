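; BlueNoise is a construction-script Blueprint that scatters instanced static meshes using what its name indicates is a blue-noise distribution.
; It initializes a seeded location container, then repeatedly requests a bounded random point, adds an instance there and records that point back into the noise data.
; Each new point is thus generated with knowledge of earlier placements.
; The random yaw range is zero, so instances share orientation and unit scale.
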(fn `UserConstructionScript`
  (locals (Location :type "Vector Structure"))
  (`BlueNoiseBPLibrary.InitLocationContainer` (`self.NoiseData`) (`self.Seed`))
  (bind _returnvalue (`AddComponent|NODE_AddInstancedStaticMeshComponent-0`))
  (for _ (range 1 (+ (`self.Count`) 1))
    (set `local.Location` (`BlueNoiseBPLibrary.MakeRandomPointInRange` (`self.NoiseData`) -450.0 450.0))
    (`InstancedStaticMeshComponent.AddInstance` _returnvalue (`KismetMathLibrary.MakeTransform` (`local.Location`) (`KismetMathLibrary.RotatorFromAxisAndAngle` (0.0 0.0 1.0) (`KismetMathLibrary.RandomFloatInRangeFromStream` 0.0 0.0 (`self.Random Locaiton`)))))
    (`BlueNoiseBPLibrary.AddLocationToNoiseData` (`self.NoiseData`) (`local.Location`))))