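; Random is a Blueprint that scatters a configurable number of instanced static mesh copies across a flat square area around its origin.
; The construction script seeds the RandomLocation stream from Seed, then adds Count instances at random X/Y offsets, giving a repeatable layout.
; Yaw reads a separate, unseeded RandomLocaiton stream with a zero range, so instances are unrotated.
; The event graph holds only disabled placeholder events.
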(fn `UserConstructionScript`
  (`KismetMathLibrary.SetRandomStreamSeed` (`self.Random Location`) (`self.Seed`))
  (bind _returnvalue (`AddComponent|NODE_AddInstancedStaticMeshComponent-0`))
  (for _ (range 1 (+ (`self.Count`) 1))
    (`InstancedStaticMeshComponent.AddInstance` _returnvalue (`KismetMathLibrary.MakeTransform` (`KismetMathLibrary.MakeVector` (`KismetMathLibrary.RandomFloatInRangeFromStream` -450.0 450.0 (`self.Random Location`)) (`KismetMathLibrary.RandomFloatInRangeFromStream` -450.0 450.0 (`self.Random Location`))) (`KismetMathLibrary.RotatorFromAxisAndAngle` (0.0 0.0 1.0) (`KismetMathLibrary.RandomFloatInRangeFromStream` 0.0 0.0 (`self.Random Locaiton`)))))))